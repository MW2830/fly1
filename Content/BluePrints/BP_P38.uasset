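; BP_P38 is a player-controllable P-38 aircraft pawn that moves on its own while the player steers its roll and pitch.
; Tick feeds movement input along world X, independent of the plane's facing, and spins the Left and Right components, likely propellers, around their roll axis using the 속도 (speed) variable.
; The Roll and Pitch input axes apply frame-time-scaled local rotations to the whole actor.
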(event `self.ReceiveTick`
  (params (DeltaSeconds :type "Float (single-precision)"))
  (`|ExecutionSequence`
    (:`then_0`
      (`self.AddMovementInput` (`KismetMathLibrary.MakeVector` (* (`GameplayStatics.GetWorldDeltaSeconds`) 500.0))))
    (:`then_1`
      (`SceneComponent.K2_AddLocalRotation` (`self.Left`) (`KismetMathLibrary.MakeRotator` (* (`GameplayStatics.GetWorldDeltaSeconds`) (`KismetMathLibrary.Conv_IntToDouble` (`self.속도`)))) false false))
    (:`then_2`
      (`SceneComponent.K2_AddLocalRotation` (`self.Right`) (`KismetMathLibrary.MakeRotator` (* (`GameplayStatics.GetWorldDeltaSeconds`) (`KismetMathLibrary.Conv_IntToDouble` (`self.속도`)))) false false))))

(event `InputAxis|Roll`
  (params (AxisValue :type "Float (single-precision)"))
  (`self.K2_AddActorLocalRotation` (`KismetMathLibrary.MakeRotator` (* (`GameplayStatics.GetWorldDeltaSeconds`) 500.0 AxisValue))))

(event `InputAxis|Pitch`
  (params (AxisValue :type "Float (single-precision)"))
  (`self.K2_AddActorLocalRotation` (`KismetMathLibrary.MakeRotator` 0.0 (* (`GameplayStatics.GetWorldDeltaSeconds`) 500.0 AxisValue))))

(fn `UserConstructionScript`)